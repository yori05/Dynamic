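; Magic circle effect actor that animates the visibility of five particle systems once at BeginPlay, then destroys itself.
; A helper function gives each valid particle system named dynamic material instances for its circle, ring and dot elements.
; A timeline then drives the Visibility scalar parameter on all of these instances together, and the actor is destroyed when it finishes.
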(event `self.ReceiveBeginPlay`
  (bind (_circle_m _ring_m _dot_m) (`self.InitializeMaterialForPS` (`self.ParticleSystem`)))
  (bind (_circle_m_2 _ring_m_2 _dot_m_2) (`self.InitializeMaterialForPS` (`self.ParticleSystem1`)))
  (bind (_circle_m_3 _ring_m_3 _dot_m_3) (`self.InitializeMaterialForPS` (`self.ParticleSystem2`)))
  (bind (_circle_m_4 _ring_m_4 _dot_m_4) (`self.InitializeMaterialForPS` (`self.ParticleSystem3`)))
  (bind (_circle_m_5 _ring_m_5 _dot_m_5) (`self.InitializeMaterialForPS` (`self.ParticleSystem4`)))
  (`self.Magic`))

(event `Magic`
  (bind (_direction _visibility_value) (`Timeline|Timeline_0`)
    (:`Update`
      (`MaterialInstanceDynamic.SetScalarParameterValue` (stale `self.ReceiveBeginPlay` _circle_m) "Visibility" _visibility_value)
      (`MaterialInstanceDynamic.SetScalarParameterValue` (stale `self.ReceiveBeginPlay` _ring_m) "Visibility" _visibility_value)
      (`MaterialInstanceDynamic.SetScalarParameterValue` (stale `self.ReceiveBeginPlay` _dot_m) "Visibility" _visibility_value)
      (`MaterialInstanceDynamic.SetScalarParameterValue` (stale `self.ReceiveBeginPlay` _circle_m_2) "Visibility" _visibility_value)
      (`MaterialInstanceDynamic.SetScalarParameterValue` (stale `self.ReceiveBeginPlay` _ring_m_2) "Visibility" _visibility_value)
      (`MaterialInstanceDynamic.SetScalarParameterValue` (stale `self.ReceiveBeginPlay` _dot_m_2) "Visibility" _visibility_value)
      (`MaterialInstanceDynamic.SetScalarParameterValue` (stale `self.ReceiveBeginPlay` _circle_m_3) "Visibility" _visibility_value)
      (`MaterialInstanceDynamic.SetScalarParameterValue` (stale `self.ReceiveBeginPlay` _ring_m_3) "Visibility" _visibility_value)
      (`MaterialInstanceDynamic.SetScalarParameterValue` (stale `self.ReceiveBeginPlay` _dot_m_3) "Visibility" _visibility_value)
      (`MaterialInstanceDynamic.SetScalarParameterValue` (stale `self.ReceiveBeginPlay` _circle_m_4) "Visibility" _visibility_value)
      (`MaterialInstanceDynamic.SetScalarParameterValue` (stale `self.ReceiveBeginPlay` _ring_m_4) "Visibility" _visibility_value)
      (`MaterialInstanceDynamic.SetScalarParameterValue` (stale `self.ReceiveBeginPlay` _dot_m_4) "Visibility" _visibility_value)
      (`MaterialInstanceDynamic.SetScalarParameterValue` (stale `self.ReceiveBeginPlay` _circle_m_5) "Visibility" _visibility_value)
      (`MaterialInstanceDynamic.SetScalarParameterValue` (stale `self.ReceiveBeginPlay` _ring_m_5) "Visibility" _visibility_value)
      (`MaterialInstanceDynamic.SetScalarParameterValue` (stale `self.ReceiveBeginPlay` _dot_m_5) "Visibility" _visibility_value))
    (:`Finished`
      (`self.K2_DestroyActor`))))

(fn `InitializeMaterialForPS`
  (params (ParticleSystem :type "PrimitiveComponent Object Reference"))
  (returns (Circle_M :type "MaterialInstanceDynamic Object Reference") (Ring_M :type "MaterialInstanceDynamic Object Reference") (Dot_M :type "MaterialInstanceDynamic Object Reference"))
  (bind _returnvalue (`KismetSystemLibrary.GetObjectName` ParticleSystem))
  (`/Engine/EditorBlueprintResources/StandardMacros.IsValid` ParticleSystem
    (:`Is Valid`
      (bind _returnvalue_2 (`PrimitiveComponent.CreateDynamicMaterialInstance` ParticleSystem 0 "/Game/Materials/MagicCircle/Magic_Circle_M.Magic_Circle_M" (`KismetStringLibrary.Conv_StringToName` (`KismetStringLibrary.Concat_StrStr` _returnvalue "_Magic_Circle_Dynamic_M"))))
      (bind _returnvalue_3 (`PrimitiveComponent.CreateDynamicMaterialInstance` ParticleSystem 1 "/Game/Materials/MagicCircle/Magic_Ring_M.Magic_Ring_M" (`KismetStringLibrary.Conv_StringToName` (`KismetStringLibrary.Concat_StrStr` _returnvalue "_Magic_Ring_Dynamic_M"))))
      (bind _returnvalue_4 (`PrimitiveComponent.CreateDynamicMaterialInstance` ParticleSystem 2 "/Game/Materials/MagicCircle/Magic_Dot_M.Magic_Dot_M" (`KismetStringLibrary.Conv_StringToName` (`KismetStringLibrary.Concat_StrStr` _returnvalue "_Magic_Dot_Dynamic_M"))))
      (return _returnvalue_2 _returnvalue_3 _returnvalue_4))
    (:`Is Not Valid`
      (return null null null))))

(fn `UserConstructionScript`)